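; Enemy pawn Blueprint that either patrols a looping list of target actors or chases the player, chosen by its State at BeginPlay.
; Patrol and Attack are self-restarting AIMoveTo loops with delays, and a failed chase falls back to patrolling.
; Tick debug-prints the target index and updates the flag that decides whether patrol advances or wraps to zero.
; An Idle event resumes patrol after a pause.
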(event Custom|Attack
  (AI|AIMoveTo self "0, 0, 0" (Game|GetPlayerCharacter 0) 5.0 false
    (:OnSuccess
      (Utilities|FlowControl|Delay 1.0)
      (CallFunction|Attack))
    (:OnFail
      (Utilities|FlowControl|Delay 0.2)
      (CallFunction|Patrol))))

(event Custom|Patrol
  (AI|AIMoveTo self "0, 0, 0" (Utilities|Array|Get(acopy) (Variables|Default|GetTargetArray) (Variables|Default|GetCurrent%20Target)) 5.0 false
    (:OnSuccess
      (if (Variables|Default|GetValue%20is%20less)
        (bind _result (Math|Integer|IncrementInt (Variables|Default|GetCurrent%20Target))
          (:%20%20
            (Variables|Default|SetCurrent%20Target _result)))
        (else
          (Variables|Default|SetCurrent%20Target 0)))
      (Utilities|FlowControl|Delay 1.0)
      (CallFunction|Patrol))))

(event Custom|Idle
  (Utilities|FlowControl|Delay 3.0)
  (CallFunction|Patrol))

(event EventBeginPlay
  (switch Utilities|FlowControl|Switch|SwitchonAiState (Variables|Default|Getstate)
    (:NewEnumerator0
      (CallFunction|Patrol))
    (:NewEnumerator1
      (CallFunction|Attack))))

(event Collision|EventActorBeginOverlap
  (params (OtherActor :type Actor%20Object%20Reference)))

(event EventTick
  (params (DeltaSeconds :type Float%20%28single-precision%29))
  (Development|PrintString (Utilities|String|ToString(Integer) (Variables|Default|GetCurrent%20Target)) true true "(R=0.000000,G=0.660000,B=1.000000,A=1.000000)" DeltaSeconds)
  (Variables|Default|SetValue%20is%20less (< (Variables|Default|GetCurrent%20Target) (- (Utilities|Array|Length (Variables|Default|GetTargetArray)) 1))))

(fn ConstructionScript)
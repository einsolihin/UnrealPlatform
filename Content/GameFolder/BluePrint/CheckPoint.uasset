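; Checkpoint actor that acts as the level's goal, unlocking once the player has collected every coin.
; BeginPlay counts all Coin actors in the level and turns off the particle effect.
; Tick compares the player's coin count to that total, showing the point light and activating particles when they match.
; With all coins collected, a player entering the box gets the game-over widget, and the in-game HUD is removed.
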(event OnComponentBeginOverlap(Box)
  (params (OverlappedComponent :type Primitive%20Component%20Object%20Reference) (OtherActor :type Actor%20Object%20Reference) (OtherComp :type Primitive%20Component%20Object%20Reference) (OtherBodyIndex :type Integer) (bFromSweep :type Boolean) (SweepResult :type Hit%20Result%20Structure%20%28by%20ref%29))
  ;[1 1 1] GameOver
  (if (== (Variables|/Game/GameFolder/BluePrint/PlayerCharacter.PlayerCharacter_C|GetCoins (stale EventTick _asplayer_character)) (Variables|Default|GetTotalCoin))
    (Utilities|Casting|CastToPlayerCharacter OtherActor)
    (bind _returnvalue (UserInterface|CreateWidget "/Game/GameFolder/BluePrint/GameOverInterface.GameOverInterface_C" (Game|GetPlayerController 0)))
    (UserInterface|Viewport|AddtoViewport _returnvalue 0)
    (Default|UIdisplay _returnvalue)
    (bind _foundwidgets (Widget|GetAllWidgetsOfClass "/Game/GameFolder/BluePrint/GameInterFace.GameInterFace_C" true))
    (Widget|RemovefromParent _foundwidgets)))

(event EventBeginPlay
  ;[1 1 1] Deactivate Check Point
  (bind _outactors (Actor|GetAllActorsOfClass "/Game/GameFolder/BluePrint/Coin.Coin_C"))
  (Variables|Default|SetTotalCoin (Utilities|Array|Length _outactors))
  (Components|Activation|Deactivate (Variables|Default|GetParticleSystem)))

(event Collision|EventActorBeginOverlap
  (params (OtherActor :type Actor%20Object%20Reference)))

(event EventTick
  (params (DeltaSeconds :type Float%20%28single-precision%29))
  ;[1 1 1] Activate the Check Point
  (bind _asplayer_character (Utilities|Casting|CastToPlayerCharacter (Game|GetPlayerCharacter 0)))
  (Development|SetHiddeninGame (Variables|Default|GetPointLight) (not (== (Variables|/Game/GameFolder/BluePrint/PlayerCharacter.PlayerCharacter_C|GetCoins _asplayer_character) (Variables|Default|GetTotalCoin))) false)
  (if (== (Variables|/Game/GameFolder/BluePrint/PlayerCharacter.PlayerCharacter_C|GetCoins _asplayer_character) (Variables|Default|GetTotalCoin))
    (Components|Activation|Activate (Variables|Default|GetParticleSystem) false)))

(fn ConstructionScript)